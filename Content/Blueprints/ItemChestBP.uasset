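; Item chest actor that opens and closes on Interact, gated by a required key card gameplay tag.
; The instigator pawn's TLActionComponent active tags are checked for an exact match; without it, a red debug message names the missing tag.
; A FlipFlop alternately plays and reverses the AnimateLid timeline, which drives lid mesh pitch and activates the particle system whenever it finishes.
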(event `SGameplayInterface.Interact`
  (params (InstigatorPawn :type "Pawn Object Reference"))
  (bind _required_key_card (`self.Required Key Card`))
  (if (`BlueprintGameplayTagLibrary.HasTag` (`TLActionComponent.ActiveGameplayTags` (`self.GetComponentByClass` InstigatorPawn "/Script/TLActionRoguelike.TLActionComponent")) _required_key_card true)
    (`/Engine/EditorBlueprintResources/StandardMacros.FlipFlop`
      (:`A`
        (bind (_direction _pitch) (`Timeline|AnimateLid` :!label _label)
          (:`Update`
            (`SceneComponent.K2_SetRelativeRotation` (`self.LidMeshComp`) (`KismetMathLibrary.MakeRotator` 0.0 _pitch) false false))
          (:`Finished`
            (`ActorComponent.Activate` (`self.ParticleSystem`) false))))
      (:`B`
        (goto _label :!via `Reverse`)))
    (else
      (`KismetSystemLibrary.PrintString` (`KismetStringLibrary.Concat_StrStr` "Missing tag: " (`BlueprintGameplayTagLibrary.GetDebugStringFromGameplayTag` _required_key_card)) true true (struct :`R` 1.0 :`G` 0.031194 :`B` 0.041141 :`A` 1.0)))))

(fn `UserConstructionScript`)